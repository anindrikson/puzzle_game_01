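; Trap cube that shoots spikes from four sides and kills the first-person player on contact.
; Tick polls the player's PhysicsObject and, when it is set and the trap is untriggered, a timeline pushes the spikes outward, re-arming after RetractDelay.
; Four Kill overlap components set the character's Dead flag, then after that delay re-arm the trap and play a second timeline that lerps the spikes back in.
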(event OnComponentBeginOverlap(kill)
  (params (OverlappedComponent :type Primitive%20Component%20Object%20Reference) (OtherActor :type Actor%20Object%20Reference) (OtherComp :type Primitive%20Component%20Object%20Reference) (OtherBodyIndex :type Integer) (bFromSweep :type Boolean) (SweepResult :type Hit%20Result%20Structure%20%28by%20ref%29))
  (bind _cube_impostor_spikes (Variables|Default|Getcube_impostor_spikes))
  (bind _cube_impostor_spikes1 (Variables|Default|Getcube_impostor_spikes1))
  (bind _cube_impostor_spikes2 (Variables|Default|Getcube_impostor_spikes2))
  (bind _cube_impostor_spikes3 (Variables|Default|Getcube_impostor_spikes3))
  (bind _asfirst_person_character (Utilities|Casting|CastToFirstPersonCharacter OtherActor))
  (Variables|/Game/FirstPersonBP/Blueprints/FirstPersonCharacter.FirstPersonCharacter_C|Setdead _asfirst_person_character true)
  (Utilities|FlowControl|Delay (Variables|Default|Getretract_delay))
  (Variables|Default|Settriggered false)
  (bind _spikes (Timeline|Timeline_1 PlayFromStart)
    (:Update
      (Transformation|SetRelativeLocation _cube_impostor_spikes (Math|Vector|MakeVector (Math|Float|Lerp (.x (Variables|/Script/Engine.SceneComponent|GetRelativeLocation _cube_impostor_spikes)) 0.0 _spikes) 0.0 0.0) false false)
      (Transformation|SetRelativeLocation _cube_impostor_spikes1 (Math|Vector|MakeVector (Math|Float|Lerp (.x (Variables|/Script/Engine.SceneComponent|GetRelativeLocation _cube_impostor_spikes1)) 0.0 _spikes) 0.0 0.0) false false)
      (Transformation|SetRelativeLocation _cube_impostor_spikes2 (Math|Vector|MakeVector 0.0 (Math|Float|Lerp (.y (Variables|/Script/Engine.SceneComponent|GetRelativeLocation _cube_impostor_spikes2)) 0.0 _spikes) 0.0) false false)
      (Transformation|SetRelativeLocation _cube_impostor_spikes3 (Math|Vector|MakeVector 0.0 (Math|Float|Lerp (.y (Variables|/Script/Engine.SceneComponent|GetRelativeLocation _cube_impostor_spikes3)) 0.0 _spikes) 0.0) false false))))

(event OnComponentBeginOverlap(kill1)
  (params (OverlappedComponent :type Primitive%20Component%20Object%20Reference) (OtherActor :type Actor%20Object%20Reference) (OtherComp :type Primitive%20Component%20Object%20Reference) (OtherBodyIndex :type Integer) (bFromSweep :type Boolean) (SweepResult :type Hit%20Result%20Structure%20%28by%20ref%29))
  (bind _cube_impostor_spikes (Variables|Default|Getcube_impostor_spikes))
  (bind _cube_impostor_spikes1 (Variables|Default|Getcube_impostor_spikes1))
  (bind _cube_impostor_spikes2 (Variables|Default|Getcube_impostor_spikes2))
  (bind _cube_impostor_spikes3 (Variables|Default|Getcube_impostor_spikes3))
  (bind _asfirst_person_character (Utilities|Casting|CastToFirstPersonCharacter OtherActor))
  (Variables|/Game/FirstPersonBP/Blueprints/FirstPersonCharacter.FirstPersonCharacter_C|Setdead _asfirst_person_character true)
  (Utilities|FlowControl|Delay (Variables|Default|Getretract_delay))
  (Variables|Default|Settriggered false)
  (bind _spikes (Timeline|Timeline_1 PlayFromStart)
    (:Update
      (Transformation|SetRelativeLocation _cube_impostor_spikes (Math|Vector|MakeVector (Math|Float|Lerp (.x (Variables|/Script/Engine.SceneComponent|GetRelativeLocation _cube_impostor_spikes)) 0.0 _spikes) 0.0 0.0) false false)
      (Transformation|SetRelativeLocation _cube_impostor_spikes1 (Math|Vector|MakeVector (Math|Float|Lerp (.x (Variables|/Script/Engine.SceneComponent|GetRelativeLocation _cube_impostor_spikes1)) 0.0 _spikes) 0.0 0.0) false false)
      (Transformation|SetRelativeLocation _cube_impostor_spikes2 (Math|Vector|MakeVector 0.0 (Math|Float|Lerp (.y (Variables|/Script/Engine.SceneComponent|GetRelativeLocation _cube_impostor_spikes2)) 0.0 _spikes) 0.0) false false)
      (Transformation|SetRelativeLocation _cube_impostor_spikes3 (Math|Vector|MakeVector 0.0 (Math|Float|Lerp (.y (Variables|/Script/Engine.SceneComponent|GetRelativeLocation _cube_impostor_spikes3)) 0.0 _spikes) 0.0) false false))))

(event OnComponentBeginOverlap(kill2)
  (params (OverlappedComponent :type Primitive%20Component%20Object%20Reference) (OtherActor :type Actor%20Object%20Reference) (OtherComp :type Primitive%20Component%20Object%20Reference) (OtherBodyIndex :type Integer) (bFromSweep :type Boolean) (SweepResult :type Hit%20Result%20Structure%20%28by%20ref%29))
  (bind _cube_impostor_spikes (Variables|Default|Getcube_impostor_spikes))
  (bind _cube_impostor_spikes1 (Variables|Default|Getcube_impostor_spikes1))
  (bind _cube_impostor_spikes2 (Variables|Default|Getcube_impostor_spikes2))
  (bind _cube_impostor_spikes3 (Variables|Default|Getcube_impostor_spikes3))
  (bind _asfirst_person_character (Utilities|Casting|CastToFirstPersonCharacter OtherActor))
  (Variables|/Game/FirstPersonBP/Blueprints/FirstPersonCharacter.FirstPersonCharacter_C|Setdead _asfirst_person_character true)
  (Utilities|FlowControl|Delay (Variables|Default|Getretract_delay))
  (Variables|Default|Settriggered false)
  (bind _spikes (Timeline|Timeline_1 PlayFromStart)
    (:Update
      (Transformation|SetRelativeLocation _cube_impostor_spikes (Math|Vector|MakeVector (Math|Float|Lerp (.x (Variables|/Script/Engine.SceneComponent|GetRelativeLocation _cube_impostor_spikes)) 0.0 _spikes) 0.0 0.0) false false)
      (Transformation|SetRelativeLocation _cube_impostor_spikes1 (Math|Vector|MakeVector (Math|Float|Lerp (.x (Variables|/Script/Engine.SceneComponent|GetRelativeLocation _cube_impostor_spikes1)) 0.0 _spikes) 0.0 0.0) false false)
      (Transformation|SetRelativeLocation _cube_impostor_spikes2 (Math|Vector|MakeVector 0.0 (Math|Float|Lerp (.y (Variables|/Script/Engine.SceneComponent|GetRelativeLocation _cube_impostor_spikes2)) 0.0 _spikes) 0.0) false false)
      (Transformation|SetRelativeLocation _cube_impostor_spikes3 (Math|Vector|MakeVector 0.0 (Math|Float|Lerp (.y (Variables|/Script/Engine.SceneComponent|GetRelativeLocation _cube_impostor_spikes3)) 0.0 _spikes) 0.0) false false))))

(event OnComponentBeginOverlap(kill3)
  (params (OverlappedComponent :type Primitive%20Component%20Object%20Reference) (OtherActor :type Actor%20Object%20Reference) (OtherComp :type Primitive%20Component%20Object%20Reference) (OtherBodyIndex :type Integer) (bFromSweep :type Boolean) (SweepResult :type Hit%20Result%20Structure%20%28by%20ref%29))
  (bind _cube_impostor_spikes (Variables|Default|Getcube_impostor_spikes))
  (bind _cube_impostor_spikes1 (Variables|Default|Getcube_impostor_spikes1))
  (bind _cube_impostor_spikes2 (Variables|Default|Getcube_impostor_spikes2))
  (bind _cube_impostor_spikes3 (Variables|Default|Getcube_impostor_spikes3))
  (bind _asfirst_person_character (Utilities|Casting|CastToFirstPersonCharacter OtherActor))
  (Variables|/Game/FirstPersonBP/Blueprints/FirstPersonCharacter.FirstPersonCharacter_C|Setdead _asfirst_person_character true)
  (Utilities|FlowControl|Delay (Variables|Default|Getretract_delay))
  (Variables|Default|Settriggered false)
  (bind _spikes (Timeline|Timeline_1 PlayFromStart)
    (:Update
      (Transformation|SetRelativeLocation _cube_impostor_spikes (Math|Vector|MakeVector (Math|Float|Lerp (.x (Variables|/Script/Engine.SceneComponent|GetRelativeLocation _cube_impostor_spikes)) 0.0 _spikes) 0.0 0.0) false false)
      (Transformation|SetRelativeLocation _cube_impostor_spikes1 (Math|Vector|MakeVector (Math|Float|Lerp (.x (Variables|/Script/Engine.SceneComponent|GetRelativeLocation _cube_impostor_spikes1)) 0.0 _spikes) 0.0 0.0) false false)
      (Transformation|SetRelativeLocation _cube_impostor_spikes2 (Math|Vector|MakeVector 0.0 (Math|Float|Lerp (.y (Variables|/Script/Engine.SceneComponent|GetRelativeLocation _cube_impostor_spikes2)) 0.0 _spikes) 0.0) false false)
      (Transformation|SetRelativeLocation _cube_impostor_spikes3 (Math|Vector|MakeVector 0.0 (Math|Float|Lerp (.y (Variables|/Script/Engine.SceneComponent|GetRelativeLocation _cube_impostor_spikes3)) 0.0 _spikes) 0.0) false false))))

(event EventBeginPlay
  (|CallParentFunction) ; This node is disabled and will not be called.\nDrag off pins to build functionality.
)

(event Collision|EventActorBeginOverlap
  (params (OtherActor :type Actor%20Object%20Reference))
  (|CallParentFunction OtherActor) ; This node is disabled and will not be called.\nDrag off pins to build functionality.
)

(event EventTick
  (params (DeltaSeconds :type Float%20%28single-precision%29))
  (|CallParentFunction DeltaSeconds)
  (bind _asfirst_person_character (Utilities|Casting|CastToFirstPersonCharacter (Game|GetPlayerCharacter 0)))
  (if (!= (Variables|/Game/FirstPersonBP/Blueprints/FirstPersonCharacter.FirstPersonCharacter_C|GetPhysicsObject _asfirst_person_character) 0)
    (if (not (Variables|Default|Gettriggered))
      (Variables|Default|Settriggered true)
      (bind _spikes (Timeline|Timeline_0 PlayFromStart)
        (:Update
          (Transformation|SetRelativeLocation (Variables|Default|Getcube_impostor_spikes) (Math|Vector|MakeVector (* _spikes -4e+01) 0.0 0.0) false false)
          (Transformation|SetRelativeLocation (Variables|Default|Getcube_impostor_spikes1) (Math|Vector|MakeVector (* _spikes 4e+01) 0.0 0.0) false false)
          (Transformation|SetRelativeLocation (Variables|Default|Getcube_impostor_spikes2) (Math|Vector|MakeVector 0.0 (* _spikes -4e+01) 0.0) false false)
          (Transformation|SetRelativeLocation (Variables|Default|Getcube_impostor_spikes3) (Math|Vector|MakeVector 0.0 (* _spikes 4e+01) 0.0) false false))
        (:Finished
          (Development|PrintString "done")
          (Utilities|FlowControl|Delay (Variables|Default|Getretract_delay))
          (Variables|Default|Settriggered false))))))

(fn ConstructionScript
  (|CallParentFunction))