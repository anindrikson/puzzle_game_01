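; Stake trap that raises its stakes when the first-person character enters its trigger and lowers them when the character leaves.
; Both overlap events act only while the Active flag is set; no damage is applied here.
; Separate timelines, one played from start and one reversed from end, drive a Lerp on the Stakes' relative Z height.
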(event OnComponentBeginOverlap(trigger)
  (params (OverlappedComponent :type Primitive%20Component%20Object%20Reference) (OtherActor :type Actor%20Object%20Reference) (OtherComp :type Primitive%20Component%20Object%20Reference) (OtherBodyIndex :type Integer) (bFromSweep :type Boolean) (SweepResult :type Hit%20Result%20Structure%20%28by%20ref%29))
  (Utilities|Casting|CastToFirstPersonCharacter OtherActor)
  (if (Variables|Default|GetActive)
    (bind _press_movement (Timeline|Timeline_0 PlayFromStart)
      (:Update
        (Transformation|SetRelativeLocation (Variables|Default|GetStakes) (Math|Vector|MakeVector 0.0 0.0 (Math|Float|Lerp 0.0 2e+02 _press_movement)) false false)))))

(event OnComponentEndOverlap(Trigger)
  (params (OverlappedComponent :type Primitive%20Component%20Object%20Reference) (OtherActor :type Actor%20Object%20Reference) (OtherComp :type Primitive%20Component%20Object%20Reference) (OtherBodyIndex :type Integer))
  (Utilities|Casting|CastToFirstPersonCharacter OtherActor)
  (if (Variables|Default|GetActive)
    (bind _press_movement (Timeline|Timeline_1 ReverseFromEnd)
      (:Update
        (Transformation|SetRelativeLocation (Variables|Default|GetStakes) (Math|Vector|MakeVector 0.0 0.0 (Math|Float|Lerp 0.0 2e+02 _press_movement)) false false)))))

(fn ConstructionScript)