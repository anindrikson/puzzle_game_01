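; BP_button is a pressure button that sinks while a companion cube or the first-person character rests on it.
; Each Tick counts those actors overlapping its Box and sets ButtonPressed, which is also set on begin overlap.
; A timeline moves ButtonBaseMesh along relative Z, playing once when pressed and reversing when the box is empty.
; Tick also prints the timeline value as debug output.
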(event OnComponentBeginOverlap(Box)
  (params (OverlappedComponent :type Primitive%20Component%20Object%20Reference) (OtherActor :type Actor%20Object%20Reference) (OtherComp :type Primitive%20Component%20Object%20Reference) (OtherBodyIndex :type Integer) (bFromSweep :type Boolean) (SweepResult :type Hit%20Result%20Structure%20%28by%20ref%29))
  (Variables|Default|Setbutton_pressed true))

(event OnComponentEndOverlap(Box)
  (params (OverlappedComponent :type Primitive%20Component%20Object%20Reference) (OtherActor :type Actor%20Object%20Reference) (OtherComp :type Primitive%20Component%20Object%20Reference) (OtherBodyIndex :type Integer)))

(event EventBeginPlay)

(event Collision|EventActorBeginOverlap
  (params (OtherActor :type Actor%20Object%20Reference)))

(event EventTick
  (params (DeltaSeconds :type Float%20%28single-precision%29))
  (Utilities|FlowControl|Sequence
    (:then_0
      (if (== (+ (Utilities|Array|Length (Collision|GetOverlappingActors (Variables|Default|GetBox) "/Game/Blueprints/BP_Companion_cube.BP_Companion_cube_C" :!class /Script/Engine.PrimitiveComponent)) (Utilities|Array|Length (Collision|GetOverlappingActors (Variables|Default|GetBox) "/Game/FirstPersonBP/Blueprints/FirstPersonCharacter.FirstPersonCharacter_C" :!class /Script/Engine.PrimitiveComponent))) 0)
        (Variables|Default|Setbutton_pressed false)
        (Variables|Default|Setanimation_playing false)
        (else
          (Variables|Default|Setbutton_pressed true)))
      (if (Variables|Default|Getbutton_pressed)
        (Utilities|FlowControl|Sequence
          (:then_0
            (if (not (Variables|Default|Getanimation_playing))
              (bind _newtrack_0 (Timeline|Timeline_0 Play)
                (:Update
                  (Transformation|SetRelativeLocation (Variables|Default|Getbutton_base_mesh) (Math|Vector|MakeVector 0.0 0.0 _newtrack_0) false false)
                  (Variables|Default|Settimeline_value _newtrack_0)))))
          (:then_1
            (Variables|Default|Setanimation_playing true)))
        (else
          (Timeline|Timeline_0 Reverse))))
    (:then_1
      (Development|PrintString (Utilities|String|ToString(Float) (Variables|Default|Gettimeline_value))))))

(fn ConstructionScript)