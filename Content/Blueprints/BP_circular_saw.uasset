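; Circular saw hazard that slices companion cubes in half and kills the player on contact.
; A timeline shuttles it 1200 units along world Y, pausing briefly before reversing at each end.
; Cutting-edge overlap with a cube plays sparks and sound, disables its gravity, then replaces it with two spawned halves.
; A cooldown flag and class check block overlapping cuts and re-cutting halves; player overlap sets Dead.
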(event OnComponentBeginOverlap(cutting_edge)
  (params (OverlappedComponent :type Primitive%20Component%20Object%20Reference) (OtherActor :type Actor%20Object%20Reference) (OtherComp :type Primitive%20Component%20Object%20Reference) (OtherBodyIndex :type Integer) (bFromSweep :type Boolean) (SweepResult :type Hit%20Result%20Structure%20%28by%20ref%29))
  (Utilities|FlowControl|Sequence
    (:then_0
      (bind _asbp_companion_cube (Utilities|Casting|CastToBP_Companion_cube OtherActor))
      (if (not (Variables|Default|Geton_cooldown))
        (if (!= (Utilities|GetClass OtherActor) "/Game/Blueprints/BP_cube_half.BP_cube_half_C")
          (Variables|Default|Seton_cooldown true)
          (bind _returnvalue (Effects|SpawnEmitteratLocation "/Game/StarterContent/Particles/P_Sparks_saw.P_Sparks_saw" (Math|Vector|MakeVector (.x (Transformation|GetWorldLocation (Variables|/Game/Blueprints/BP_Companion_cube.BP_Companion_cube_C|Getcube_mesh _asbp_companion_cube))) (.y (Transformation|GetWorldLocation (Variables|/Game/Blueprints/BP_Companion_cube.BP_Companion_cube_C|Getcube_mesh _asbp_companion_cube))) (+ (.z (Transformation|GetWorldLocation (Variables|/Game/Blueprints/BP_Companion_cube.BP_Companion_cube_C|Getcube_mesh _asbp_companion_cube))) 45.0))))
          (Audio|PlaySoundatLocation "/Game/Sounds/circular_saw.circular_saw" (Transformation|GetWorldLocation (Variables|/Game/Blueprints/BP_Companion_cube.BP_Companion_cube_C|Getcube_mesh _asbp_companion_cube)) "0, 0, 0" 1.0 1.0 0.0 0 0 0)
          (Utilities|FlowControl|Delay 0.2)
          (Physics|SetEnableGravity (Variables|/Game/Blueprints/BP_Companion_cube.BP_Companion_cube_C|Getcube_mesh _asbp_companion_cube) false)
          (Collision|SetCollisionResponsetoChannel (Variables|/Game/Blueprints/BP_Companion_cube.BP_Companion_cube_C|Getcube_mesh _asbp_companion_cube) "ECC_WorldDynamic" "ECR_Ignore")
          (Utilities|FlowControl|Delay 0.5)
          (Game|SpawnActorfromClass "/Game/Blueprints/BP_cube_half.BP_cube_half_C" (Math|Transform|MakeTransform (Math|Vector|MakeVector (+ (.x (Transformation|GetWorldLocation (Variables|/Game/Blueprints/BP_Companion_cube.BP_Companion_cube_C|Getcube_mesh _asbp_companion_cube))) 3e+01) (.y (Transformation|GetWorldLocation (Variables|/Game/Blueprints/BP_Companion_cube.BP_Companion_cube_C|Getcube_mesh _asbp_companion_cube))) (.z (Transformation|GetWorldLocation (Variables|/Game/Blueprints/BP_Companion_cube.BP_Companion_cube_C|Getcube_mesh _asbp_companion_cube)))) "0.000000,270.000000,0.000000" "1,1,1") "AdjustIfPossibleButAlwaysSpawn" 0 0)
          (Game|SpawnActorfromClass "/Game/Blueprints/BP_cube_half.BP_cube_half_C" (Math|Transform|MakeTransform (Math|Vector|MakeVector (- (.x (Transformation|GetWorldLocation (Variables|/Game/Blueprints/BP_Companion_cube.BP_Companion_cube_C|Getcube_mesh _asbp_companion_cube))) 3e+01) (.y (Transformation|GetWorldLocation (Variables|/Game/Blueprints/BP_Companion_cube.BP_Companion_cube_C|Getcube_mesh _asbp_companion_cube))) (.z (Transformation|GetWorldLocation (Variables|/Game/Blueprints/BP_Companion_cube.BP_Companion_cube_C|Getcube_mesh _asbp_companion_cube)))) "0,90.000000,0.000000" "1,1,1") "AdjustIfPossibleButAlwaysSpawn" 0 0)
          (Actor|DestroyActor _asbp_companion_cube)
          (Components|DestroyComponent _returnvalue)
          (Variables|Default|Seton_cooldown false))))
    (:then_1
      (bind _asfirst_person_character (Utilities|Casting|CastToFirstPersonCharacter OtherActor))
      (Variables|/Game/FirstPersonBP/Blueprints/FirstPersonCharacter.FirstPersonCharacter_C|Setdead _asfirst_person_character true))))

(event EventBeginPlay
  (Variables|Default|Setinitial_location (Transformation|GetActorLocation))
  (bind _movement (Timeline|Timeline_0 Play)
    (:Update
      (Transformation|SetActorLocation (Math|Vector|MakeVector (.x (Variables|Default|Getinitial_location)) (+ (.y (Variables|Default|Getinitial_location)) (* _movement 1.2e+03)) (.z (Variables|Default|Getinitial_location))) false false))
    (:Finished
      (Utilities|FlowControl|Delay 0.5)
      (if (Math|Vector|Equal(Vector) (Transformation|GetActorLocation) (Variables|Default|Getinitial_location) 0.0001)
        (Timeline|Timeline_0 PlayFromStart)
        (else
          (Timeline|Timeline_0 ReverseFromEnd))))))

(event Collision|EventActorBeginOverlap
  (params (OtherActor :type Actor%20Object%20Reference)))

(event EventTick
  (params (DeltaSeconds :type Float%20%28single-precision%29)))

(fn ConstructionScript)