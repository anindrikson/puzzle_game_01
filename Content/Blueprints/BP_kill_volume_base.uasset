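; Base kill volume that kills the player or respawns companion cubes when they enter it.
; While active, its Volume component's begin-overlap event runs two independently toggled checks on the overlapping actor.
; A first-person character gets its death index set from the configured death type and is flagged dead.
; A companion cube is told to respawn itself.
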(event OnComponentBeginOverlap(volume)
  (params (OverlappedComponent :type Primitive%20Component%20Object%20Reference) (OtherActor :type Actor%20Object%20Reference) (OtherComp :type Primitive%20Component%20Object%20Reference) (OtherBodyIndex :type Integer) (bFromSweep :type Boolean) (SweepResult :type Hit%20Result%20Structure%20%28by%20ref%29))
  (if (Variables|Default|Getactive)
    (Utilities|FlowControl|Sequence
      (:then_0
        (if (Variables|Default|Getkill_player)
          (bind _asfirst_person_character (Utilities|Casting|CastToFirstPersonCharacter OtherActor))
          (Variables|/Game/FirstPersonBP/Blueprints/FirstPersonCharacter.FirstPersonCharacter_C|Setdeath_index _asfirst_person_character (Variables|Default|Getdeath_type))
          (Variables|/Game/FirstPersonBP/Blueprints/FirstPersonCharacter.FirstPersonCharacter_C|Setdead _asfirst_person_character true)))
      (:then_1
        (if (Variables|Default|Getkill_cube)
          (bind _asbp_companion_cube (Utilities|Casting|CastToBP_Companion_cube OtherActor))
          (Default|RespawnCube _asbp_companion_cube))))))

(event EventBeginPlay)

(event Collision|EventActorBeginOverlap
  (params (OtherActor :type Actor%20Object%20Reference)))

(event EventTick
  (params (DeltaSeconds :type Float%20%28single-precision%29)))

(fn ConstructionScript)