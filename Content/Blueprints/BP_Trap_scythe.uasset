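; BP_Trap_scythe is a trap Blueprint that swings a scythe when the FirstPersonCharacter overlaps its trigger.
; The overlap looks up the BP_Companion_cube actor and proceeds only if an Activate flag is set.
; A timeline then plays from the start, lerping the scythe's relative pitch through a quarter turn.
; Two alternative rotation and location movement nodes are left unconnected.
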(event OnComponentBeginOverlap(trigger)
  (params (OverlappedComponent :type Primitive%20Component%20Object%20Reference) (OtherActor :type Actor%20Object%20Reference) (OtherComp :type Primitive%20Component%20Object%20Reference) (OtherBodyIndex :type Integer) (bFromSweep :type Boolean) (SweepResult :type Hit%20Result%20Structure%20%28by%20ref%29))
  (Utilities|Casting|CastToFirstPersonCharacter OtherActor)
  (Actor|GetActorOfClass "/Game/Blueprints/BP_Companion_cube.BP_Companion_cube_C")
  (if (Variables|Default|GetActivate)
    (bind _press_movement (Timeline|Timeline_0 PlayFromStart)
      (:Update
        (Transformation|SetRelativeRotation (Variables|Default|GetScythe) (Math|Rotator|MakeRotator 0.0 (Math|Float|Lerp 0.0 -9e+01 _press_movement) 0.0) false false)))))

(fn ConstructionScript)