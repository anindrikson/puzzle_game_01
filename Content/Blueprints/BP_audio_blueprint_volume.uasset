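; Trigger volume actor that plays an assignable sound when something overlaps its box.
; With Recurring set, each entry restarts the sound; otherwise it plays on the first entry and later entries only fade the volume back up.
; Leaving the box fades the audio to near silence without stopping it.
; Overlaps are not filtered by actor.
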(event OnComponentBeginOverlap(Box)
  (params (OverlappedComponent :type Primitive%20Component%20Object%20Reference) (OtherActor :type Actor%20Object%20Reference) (OtherComp :type Primitive%20Component%20Object%20Reference) (OtherBodyIndex :type Integer) (bFromSweep :type Boolean) (SweepResult :type Hit%20Result%20Structure%20%28by%20ref%29))
  (bind _audio (Variables|Default|Getaudio))
  (if (Variables|Default|Getrecurring)
    (Audio|Components|Audio|SetSound _audio (Variables|Default|Getsound_to_play) :!label _label)
    (Audio|Components|Audio|Play _audio 0.0)
    (Variables|Default|Setplayed true)
    (elif (Variables|Default|Getplayed)
      (Audio|Components|Audio|AdjustVolume (Variables|Default|Getaudio) 0.6 1.0 "Linear" :!class /Script/Engine.AudioComponent)
      (else
        (goto _label)))))

(event OnComponentEndOverlap(Box)
  (params (OverlappedComponent :type Primitive%20Component%20Object%20Reference) (OtherActor :type Actor%20Object%20Reference) (OtherComp :type Primitive%20Component%20Object%20Reference) (OtherBodyIndex :type Integer))
  (Audio|Components|Audio|AdjustVolume (Variables|Default|Getaudio) 0.8 0.0001 "Linear" :!class /Script/Engine.AudioComponent))

(event EventBeginPlay)

(event Collision|EventActorBeginOverlap
  (params (OtherActor :type Actor%20Object%20Reference)))

(event EventTick
  (params (DeltaSeconds :type Float%20%28single-precision%29)))

(fn ConstructionScript)