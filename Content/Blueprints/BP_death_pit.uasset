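; BP_death_pit is a pit whose Floor opens or closes according to an associated BP_button.
; Every Tick it polls the button's ButtonPressed state and compares it with FlipLogic, which inverts the behavior.
; When the two differ, the Floor turns invisible and ignores all collision channels; otherwise it is visible and blocks them.
; The graph itself contains no damage or kill logic.
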(event EventBeginPlay)

(event Collision|EventActorBeginOverlap
  (params (OtherActor :type Actor%20Object%20Reference)))

(event EventTick
  (params (DeltaSeconds :type Float%20%28single-precision%29))
  (bind _floor (Variables|Default|Getfloor))
  (bind _associated_button (Variables|Default|Getassociated_button)
    (:then
      (bind _asbp_button (Utilities|Casting|CastToBP_button _associated_button))
      (if (Math|Boolean|NotEqual(Boolean) (Variables|Default|Getflip_logic) (Variables|/Game/Blueprints/BP_button.BP_button_C|Getbutton_pressed _asbp_button))
        (Rendering|SetVisibility _floor false false)
        (Collision|SetCollisionResponsetoAllChannels _floor "ECR_Ignore")
        (else
          (Rendering|SetVisibility _floor true false)
          (Collision|SetCollisionResponsetoAllChannels _floor "ECR_Block"))))
    (:else)))

(fn ConstructionScript)