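; BP_Companion_cube is a companion cube actor that can respawn at its starting position.
; It records its location in the construction script and on BeginPlay.
; The respawn_cube event plays an explosion emitter and sound at the cube mesh's location, spawns a fresh copy of its own class at the saved start, then destroys itself.
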(event Custom|respawn_cube
  (bind _self self)
  (bind _cube_mesh (Variables|Default|Getcube_mesh _self))
  (bind _returnvalue (Transformation|GetWorldLocation _cube_mesh))
  (Effects|SpawnEmitteratLocation "/Game/StarterContent/Particles/P_Explosion.P_Explosion" _returnvalue)
  (Audio|PlaySoundatLocation "/Game/Sounds/explosion.explosion" _returnvalue "0, 0, 0" 1.0 1.0 0.0 0 0 0)
  (Game|SpawnActorfromClass (Utilities|GetClass self) (Math|Transform|MakeTransform (Variables|Default|Getstart_location) "0, 0, 0" "1,1,1") "Undefined" 0 0)
  (Actor|DestroyActor))

(event EventBeginPlay
  (Variables|Default|Setstart_location (Transformation|GetActorLocation)))

(event Collision|EventActorBeginOverlap
  (params (OtherActor :type Actor%20Object%20Reference)))

(event EventTick
  (params (DeltaSeconds :type Float%20%28single-precision%29)))

(fn ConstructionScript
  (Variables|Default|Setstart_location (Transformation|GetActorLocation)))