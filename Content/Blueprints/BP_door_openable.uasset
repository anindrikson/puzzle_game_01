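; BP_door_openable is a sliding door that moves its mesh along relative Y, driven by either a trigger volume or a linked button.
; With UseTriggerVolume on, a player overlap plays a timeline and an opening sound scaled by the character's MasterVolume, and leaving reverses the timeline.
; With it off, Tick polls the associated BP_button's TimelineValue to position the mesh.
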(event OnComponentBeginOverlap(trigger)
  (params (OverlappedComponent :type Primitive%20Component%20Object%20Reference) (OtherActor :type Actor%20Object%20Reference) (OtherComp :type Primitive%20Component%20Object%20Reference) (OtherBodyIndex :type Integer) (bFromSweep :type Boolean) (SweepResult :type Hit%20Result%20Structure%20%28by%20ref%29))
  (bind _asfirst_person_character (Utilities|Casting|CastToFirstPersonCharacter OtherActor))
  (if (Variables|Default|Getuse_trigger_volume)
    (Audio|PlaySoundatLocation "/Game/Sounds/Open_door.Open_door" "0, 0, 0" "0, 0, 0" (Variables|/Game/FirstPersonBP/Blueprints/FirstPersonCharacter.FirstPersonCharacter_C|Getmaster_volume _asfirst_person_character) 1.0 0.0 0 0 0)
    (bind _newtrack_0 (Timeline|Timeline_0 PlayFromStart)
      (:Update
        (Transformation|SetRelativeLocation (Variables|Default|Getdoor_mesh) (Math|Vector|MakeVector 0.0 (* _newtrack_0 14.0) 0.0) false false)))))

(event OnComponentEndOverlap(trigger)
  (params (OverlappedComponent :type Primitive%20Component%20Object%20Reference) (OtherActor :type Actor%20Object%20Reference) (OtherComp :type Primitive%20Component%20Object%20Reference) (OtherBodyIndex :type Integer))
  (Utilities|Casting|CastToFirstPersonCharacter OtherActor)
  (if (Variables|Default|Getuse_trigger_volume)
    (bind _newtrack_0 (Timeline|Timeline_0 ReverseFromEnd)
      (:Update
        (Transformation|SetRelativeLocation (Variables|Default|Getdoor_mesh) (Math|Vector|MakeVector 0.0 (* _newtrack_0 14.0) 0.0) false false)))))

(event EventBeginPlay)

(event Collision|EventActorBeginOverlap
  (params (OtherActor :type Actor%20Object%20Reference)))

(event EventTick
  (params (DeltaSeconds :type Float%20%28single-precision%29))
  (if (not (Variables|Default|Getuse_trigger_volume))
    (bind _associated_button (Variables|Default|Getassociated_button)
      (:then
        (bind _asbp_button (Utilities|Casting|CastToBP_button _associated_button))
        (Transformation|SetRelativeLocation (Variables|Default|Getdoor_mesh) (Math|Vector|MakeVector 0.0 (* (Variables|/Game/Blueprints/BP_button.BP_button_C|Gettimeline_value _asbp_button) 14.0) 0.0) false false))
      (:else))))

(fn ConstructionScript)